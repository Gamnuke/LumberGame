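; TreeBPExample is a scratch Blueprint for Procedural Mesh experiments that does nothing in game, as BeginPlay and the construction script are empty.
; One disconnected chain repeatedly builds a two-quad, rock-material strip from hardcoded vertices and draws debug points.
; Another builds a triangle from Vertexes, using a normalized edge cross product as its flat normal and drawing that as a debug line.
; Stray line trace and mesh-update nodes are also unwired.
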(event `self.ReceiveBeginPlay`)

(fn `UserConstructionScript`)